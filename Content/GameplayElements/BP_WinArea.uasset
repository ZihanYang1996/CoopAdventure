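; BP_WinArea handles winning the game, responding when its win condition is met.
; On BeginPlay it binds GameWon to the OnWinConditionMet event; the condition itself is evaluated outside this graph.
; GameWon disables the first player's pawn input, waits briefly, then shows the WBP_WinScreen widget with the mouse cursor and UI-only input.
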(event Custom|GameWon
  (bind _returnvalue (Game|GetPlayerController 0))
  (Input|DisableInput (Game|Player|GetPlayerPawn 0) (Game|GetPlayerController 0))
  (Utilities|FlowControl|Delay 2.0)
  (bind _returnvalue_2 (UserInterface|CreateWidget "/Game/GameplayElements/WBP_WinScreen.WBP_WinScreen_C"))
  (UserInterface|Viewport|AddtoViewport _returnvalue_2 0)
  (Variables|/Script/Engine.PlayerController|SetbShowMouseCursor _returnvalue true)
  (Input|SetInputModeUIOnly _returnvalue 0 "DoNotLock" false))

(event EventBeginPlay
  (EventDispatchers|BindEventtoOnWinConditionMet (delegate Custom|GameWon)))

(fn ConstructionScript)